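; Player controller that lets the user pick a feature in a Cesium 3D Tileset by left mouse double-click and report its "pnu" ID to a REST API.
; On a valid face hit, it stores the tileset tagged PNU_SELECTED and reads the face's pnu metadata from the hit component.
; An async HTTP request sends that value in the URL, marked as a TODO, and its callback refreshes the stored tileset.
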(event `self.ReceiveBeginPlay`
  (add `self.LeftMouseDoubleClick` (delegate `LeftMouseDoubleClick_Event_0`)))

(event `LeftMouseDoubleClick_Event_0` :!signature `self.LeftMouseDoubleClick`
  (params (ScreenPos :type "Vector2D Structure (by ref)") (HitResult :type "HitResult Structure (by ref)"))
  (bind (_bblockinghit _binitialoverlap _time _distance _location _impactpoint _normal _impactnormal _physmat _hitactor _hitcomponent _hitbonename _hititem _elementindex _faceindex) (`GameplayStatics.BreakHitResult` HitResult))
  (`/Engine/EditorBlueprintResources/StandardMacros.CompareInt` _faceindex
    (:`>`
      (`KismetSystemLibrary.PrintString` "FINDING TILESET" true true (struct :`R` 0.337606 :`B` 1.0 :`A` 1.0) 5.0 :!label _label)
      ;[1 1 1] Save the tileset reference of the selected PNU.
      (bind _outactors (`GameplayStatics.GetAllActorsOfClassWithTag` "/Script/CesiumRuntime.Cesium3DTileset" "PNU_SELECTED"))
      (`/Engine/EditorBlueprintResources/StandardMacros.CompareInt` (`KismetArrayLibrary.Array_Length` _outactors)
        (:`>`
          (for _array_element _outactors
            (set `self.selctedTileset` _array_element))
          (`EleventhLibrary.AsyncHttp` (delegate `CustomEvent_0`) (`KismetStringLibrary.Concat_StrStr` (`self.url`) "/" (`BlueprintMapLibrary.Map_Find` (`CesiumMetadataUtilityBlueprintLibrary.GetMetadataValuesAsStringForFace` _hitcomponent (`KismetMathLibrary.Conv_IntToInt64` _faceindex)) "pnu"))))
        (:`==`
          (`KismetSystemLibrary.PrintString` "FAILED TO FIND" true true (struct :`R` 1.0 :`G` 0.020309 :`B` 0.010362 :`A` 1.0) 5.0 :!label _label_2))
        (:`<`
          (goto _label_2))))
    (:`==`
      (goto _label))
    (:`<`
      (`KismetSystemLibrary.PrintString` "INVALID FACEINDEX" true true (struct :`R` 0.337606 :`B` 1.0 :`A` 1.0) 5.0))))

(event `CustomEvent_0`
  (params (result :type Boolean))
  (`Cesium3DTileset.RefreshTileset` (`self.selctedTileset`)))

(fn `NewFunction_0`)

(fn `UserConstructionScript`)